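; BP_DoorSwitch is an interactable switch that removes its assigned doors when used.
; It overrides interaction hooks from its parent class, accepting any valid interactor and passing interaction attempts straight to the parent.
; On a successful interaction it loops through the SelectedDoor array and destroys each valid actor, so the doors are removed outright rather than animated open.
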(fn `CheckIfInteractionValid`
  (params (Interactor :type "Actor Object Reference"))
  (returns (`Has Output` :type Boolean))
  (`/Engine/EditorBlueprintResources/StandardMacros.IsValid` Interactor
    (:`Is Valid`
      (return true))
    (:`Is Not Valid`
      (return false))))

(fn `OnInteractionAttempt`
  (params (Interactor :type "Actor Object Reference"))
  (`parent.OnInteractionAttempt` Interactor))

(fn `OnSuccessInteraction`
  (params (Interactor :type "Actor Object Reference"))
  (for _array_element (`self.SelectedDoor`)
    (`/Engine/EditorBlueprintResources/StandardMacros.IsValid` _array_element
      (:`Is Valid`
        (`self.K2_DestroyActor` _array_element)))))

(fn `UserConstructionScript`
  (`parent.UserConstructionScript`))