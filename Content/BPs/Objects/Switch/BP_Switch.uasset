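; BP_Switch is an interactable switch that relays an interaction to a set of other interactables.
; TryToInteract accepts every attempt unconditionally by sending itself the SuccessfulInteract message.
; SuccessfulInteract loops over the SelectedInteractables set and sends TryToInteract to each valid entry, passing the original Interactor along.
; Communication runs through interface-style messages, so the switch needs no knowledge of what each target does.
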(event `self.TryToInteract`
  (params (Interactor :type "Actor Object Reference"))
  (message `iInteractable.Successful_Interact` self Interactor))

(event `self.Successful_Interact`
  (params (Interactor :type "Actor Object Reference"))
  (bind _valuepin (`|SetForEach` (`self.SelectedInteractables`))
    (:`then`
      (`/Engine/EditorBlueprintResources/StandardMacros.IsValid` _valuepin
        (:`Is Valid`
          (message `iInteractable.TryToInteract` _valuepin Interactor))))))

(fn `UserConstructionScript`
  (`parent.UserConstructionScript`))