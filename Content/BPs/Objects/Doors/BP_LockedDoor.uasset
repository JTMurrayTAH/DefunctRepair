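; BP_LockedDoor is a lockable door that only opens for an interactor while unlocked.
; TrytoInteract forwards to InteractionLogic, which checks LockedState and either plays a denied sound with a "Locked" debug print, or runs the inherited DoorInteraction.
; Lock and Unlock events toggle the state, while the door behavior itself comes from the parent class.
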(event `self.TryToInteract`
  (params (Interactor :type "Actor Object Reference"))
  (message `iInteractable.Interaction_Logic` self Interactor))

(event `self.Interaction_Logic`
  (params (Interactor :type "Actor Object Reference"))
  (bind _returnvalue (`cpp_ILockable.isLocked`))
  (if _returnvalue
    (`iInteractable.Failed_Interact` Interactor)
    (`GameplayStatics.PlaySoundAtLocation` "/Game/Sounds/DoorLocked_Denied_Cue.DoorLocked_Denied_Cue" (`self.K2_GetActorLocation`) (struct) 1.0 1.0 0.0 null null null null)
    (else
      (`iInteractable.Successful_Interact` Interactor))))

(event `self.Failed_Interact`
  (params (Interactor :type "Actor Object Reference"))
  (`KismetSystemLibrary.PrintString` "Locked"))

(event `self.Successful_Interact`
  (params (Interactor :type "Actor Object Reference"))
  (`self.DoorInteraction`))

(event `self.unlock`
  (set `self.LockedState` false))

(event `self.lock`
  (set `self.LockedState` true))

(fn `DoorInteraction`
  (`parent.DoorInteraction`)
  (return))

(fn `isLocked`
  (returns (ReturnValue :type Boolean))
  (return (`self.LockedState`)))

(fn `UserConstructionScript`
  (`parent.UserConstructionScript`))