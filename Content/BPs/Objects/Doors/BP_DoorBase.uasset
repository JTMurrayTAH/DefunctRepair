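; BP_DoorBase is a door actor, apparently a base class, that opens and closes by disappearing and reappearing rather than animating.
; DoorInteraction toggles IsOpen: opening hides the whole actor and disables its collision, while closing restores both.
; It prints the new state for debugging.
; The event graph and construction script are empty, and nothing in this file calls DoorInteraction.
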(fn `DoorInteraction`
  (if (`self.IsOpen`)
    (`self.SetActorHiddenInGame` false)
    (`self.SetActorEnableCollision` true)
    (else
      (`self.SetActorHiddenInGame` true)
      (`self.SetActorEnableCollision` false)))
  (bind _output_get (set `self.IsOpen` (not (`self.IsOpen`))))
  (`KismetSystemLibrary.PrintString` (`KismetStringLibrary.Conv_BoolToString` _output_get)))

(fn `UserConstructionScript`)