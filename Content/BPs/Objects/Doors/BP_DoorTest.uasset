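; BP_DoorTest is a test door actor that toggles between open and closed when interacted with.
; TrytoInteract passes the interactor straight to SuccessfulInteract without any checks, which then calls DoorInteraction.
; DoorInteraction fakes opening by hiding the actor and disabling its collision, restores both to close, then flips IsOpen and prints the new state.
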(event `self.TryToInteract`
  (params (Interactor :type "Actor Object Reference"))
  (`iInteractable.Successful_Interact` Interactor))

(event `self.Successful_Interact`
  (params (Interactor :type "Actor Object Reference"))
  (`self.DoorInteraction`))

(fn `DoorInteraction`
  (if (`self.IsOpen`)
    (`self.SetActorHiddenInGame` false)
    (`self.SetActorEnableCollision` true)
    (else
      (`self.SetActorHiddenInGame` true)
      (`self.SetActorEnableCollision` false)))
  (bind _output_get (set `self.IsOpen` (not (`self.IsOpen`))))
  (`KismetSystemLibrary.PrintString` (`KismetStringLibrary.Conv_BoolToString` _output_get)))

(fn `UserConstructionScript`)