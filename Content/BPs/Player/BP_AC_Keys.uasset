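; Player actor component that tracks how many keys of each level the player holds.
; Counts live in the KeyInventory map, indexed by key level clamped to a fixed range of tiers.
; AddKey increments the count for a level and writes it back to the map.
; RemoveKey decrements it only when that count is non-zero, and nothing runs on BeginPlay or Tick.
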(event `AddKey`
  (params (KeyLevel :type Integer))
  (bind _returnvalue (`KismetMathLibrary.Clamp` KeyLevel 0 4))
  (bind _keyinventory (`self.KeyInventory`))
  (bind _result (`/Engine/EditorBlueprintResources/StandardMacros.IncrementInt` (`BlueprintMapLibrary.Map_Find` _keyinventory _returnvalue))
    (:`  `
      (`BlueprintMapLibrary.Map_Add` _keyinventory _returnvalue _result))))

(event `RemoveKey`
  (params (KeyLevel :type Integer))
  (bind _returnvalue (`KismetMathLibrary.Clamp` KeyLevel 0 4))
  (bind _keyinventory (`self.KeyInventory`))
  (bind _value (`BlueprintMapLibrary.Map_Find` _keyinventory _returnvalue))
  (if (!= _value 0)
    (bind _result (`/Engine/EditorBlueprintResources/StandardMacros.DecrementInt` _value)
      (:`  `
        (`BlueprintMapLibrary.Map_Add` _keyinventory _returnvalue _result)))))