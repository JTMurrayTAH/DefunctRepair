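; BP_Player is the first-person player character, with movement, jumping, looking, two-handed grabbing for climbing, and interaction.
; On BeginPlay it binds to movement, jump and look input events from BP_DrPController.
; Primary and secondary Enhanced Input actions drive left and right hand grab and release on BPACClimb, using the camera as origin.
; Interact line-traces from the camera and messages hit actors implementing IInteractable.
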(event `self.ReceiveBeginPlay`
  (`self.BindEvents`))

(event `self.ReceiveTick`
  (params (DeltaSeconds :type "Float (single-precision)")))

(event `EnhancedInput|/Game/BPs/Player/input/IA/Standard/IA_UsePrimary`
  (params (ActionValue :type Boolean) (ElapsedSeconds :type "Float (double-precision)") (TriggeredSeconds :type "Float (double-precision)") (InputAction :type "InputAction Object Reference" :default "/Game/BPs/Player/input/IA/Standard/IA_UsePrimary.IA_UsePrimary"))
  (bind _bp_ac_climb (`self.BP_AC_Climb`))
  (:`Started`
    (`/Game/BPs/Player/BP_AC_Climb.LeftHandGrab` _bp_ac_climb (`self.PlayerCamera`) 250.0))
  (:`Canceled`
    (`/Game/BPs/Player/BP_AC_Climb.LeftHandRelease` _bp_ac_climb :!label _label))
  (:`Completed`
    (goto _label)))

(event `EnhancedInput|/Game/BPs/Player/input/IA/Standard/IA_UseSecondary`
  (params (ActionValue :type Boolean) (ElapsedSeconds :type "Float (double-precision)") (TriggeredSeconds :type "Float (double-precision)") (InputAction :type "InputAction Object Reference" :default "/Game/BPs/Player/input/IA/Standard/IA_UseSecondary.IA_UseSecondary"))
  (bind _bp_ac_climb (`self.BP_AC_Climb`))
  (:`Started`
    (`/Game/BPs/Player/BP_AC_Climb.RightHandGrab` _bp_ac_climb 250.0 (`self.PlayerCamera`)))
  (:`Canceled`
    (`/Game/BPs/Player/BP_AC_Climb.RightHandRelease` _bp_ac_climb :!label _label_2))
  (:`Completed`
    (goto _label_2)))

(event `EnhancedInput|/Game/BPs/Player/input/IA/Standard/IA_Interact`
  (params (ActionValue :type Boolean) (ElapsedSeconds :type "Float (double-precision)") (TriggeredSeconds :type "Float (double-precision)") (InputAction :type "InputAction Object Reference" :default "/Game/BPs/Player/input/IA/Standard/IA_Interact.IA_Interact"))
  (bind _playercamera (`self.PlayerCamera`))
  (bind _returnvalue (`SceneComponent.K2_GetComponentLocation` _playercamera))
  (:`Triggered`
    (bind (_outhit _returnvalue_2) (`KismetSystemLibrary.LineTraceSingle` :`Start` _returnvalue :`End` (+ _returnvalue (* (`SceneComponent.GetForwardVector` _playercamera) 250.0)) :`TraceChannel` "TraceTypeQuery1" :`DrawDebugType` "ForDuration"))
    (if _returnvalue_2
      (bind (_bblockinghit _binitialoverlap _time _distance _location _impactpoint _normal _impactnormal _physmat _hitactor) (`GameplayStatics.BreakHitResult` _outhit))
      (if (`KismetSystemLibrary.DoesImplementInterface` _hitactor "/Script/DR.iInteractable")
        (message `iInteractable.TryToInteract` _hitactor self)))))

(fn `BindEvents`
  (bind _asbp_dr_pcontroller (cast `/Game/BPs/Gamemode/BP_DrPController` (`GameplayStatics.GetPlayerController` 0)))
  (add `Cpp_DrPController.OnMovementInput` _asbp_dr_pcontroller (`|CreateDelegate` :!event `MovementFunc`))
  (add `Cpp_DrPController.OnJumpInput` _asbp_dr_pcontroller (`|CreateDelegate` :!event `Jump`))
  (add `Cpp_DrPController.OnLookInput` _asbp_dr_pcontroller (`|CreateDelegate` :!event `LookFunc`)))

(fn `JumpFunc`
  (`self.Jump`))

(fn `LookFunc`
  (params (`V2 Input` :type "Vector2D Structure"))
  (`self.AddControllerPitchInput` (/ `V2 Input_Y` -1.0))
  (`self.AddControllerYawInput` `V2 Input_X`))

(fn `MovementFunc`
  (params (`V2 Input` :type "Vector2D Structure"))
  (`self.AddMovementInput` (`self.GetActorRightVector`) `V2 Input_X`)
  (`self.AddMovementInput` (`self.GetActorForwardVector`) `V2 Input_Y`))

(fn `UserConstructionScript`)