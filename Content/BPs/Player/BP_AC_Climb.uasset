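; Climbing component that lets BP_Player pull itself toward surfaces grabbed with either hand.
; Each grab line-traces forward from a supplied component and stores the hit location if its physical material is PM_Climbable.
; A zero vector means a free hand.
; Every tick, each held point adds a movement force toward it that grows with distance, plus a base grab force, with extra vertical weighting.
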(event `self.ReceiveBeginPlay`
  (bind _returnvalue (`GameplayStatics.GetActorOfClass` "/Game/BPs/Player/BP_Player.BP_Player_C"))
  (set `self.Player` _returnvalue))

(event `self.ReceiveTick`
  (params (DeltaSeconds :type "Float (single-precision)"))
  (if (or (!= (`self.LeftHand_Loc`) (0.0 0.0 0.0)) (!= (`self.RightHand_Loc`) (0.0 0.0 0.0)))
    (set `self.IsClimbing` true)
    (else
      (set `self.IsClimbing` false)))
  (`self.Climb Function`))

(fn `Climb Function`
  (bind _righthand_loc (`self.RightHand_Loc`))
  (bind _lefthand_loc (`self.LeftHand_Loc`))
  (bind _returnvalue (`Actor.K2_GetActorLocation` (`self.Player`)))
  (bind _returnvalue_2 (`Actor.K2_GetActorLocation` (`self.Player`)))
  (if (`self.IsClimbing`)
    (if (!= _lefthand_loc (0.0 0.0 0.0))
      (`CharacterMovementComponent.AddForce` (`Character.CharacterMovement` (`self.Player`)) (* (* (- _lefthand_loc _returnvalue) (+ (`KismetMathLibrary.Vector_Distance` _lefthand_loc _returnvalue) (`self.PlayerBaseGrabForce`))) (1.0 1.0 1.5))))
    (if (!= _righthand_loc (0.0 0.0 0.0))
      (`CharacterMovementComponent.AddForce` (`Character.CharacterMovement` (`self.Player`)) (* (* (- _righthand_loc _returnvalue_2) (+ (`KismetMathLibrary.Vector_Distance` _righthand_loc _returnvalue_2) (`self.PlayerBaseGrabForce`))) (1.0 1.2 1.5))))))

(fn `LeftHandGrab`
  (params (`Origin Component` :type "SceneComponent Object Reference") (`Grab Length` :type "Float (single-precision)"))
  (bind _grab_point (`self.RayCast` `Origin Component` `Grab Length`))
  (`self.Set LeftHand` _grab_point)
  (return))

(fn `LeftHandRelease`
  (`self.Set LeftHand` (0.0 0.0 0.0))
  (return))

(fn `RayCast`
  (params (`Origin Component` :type "SceneComponent Object Reference") (`Grab Length` :type "Float (single-precision)"))
  (returns (`Grab Point` :type "Vector Structure"))
  (bind _returnvalue (`SceneComponent.K2_GetComponentLocation` `Origin Component`))
  (bind (_outhit _returnvalue_2) (`KismetSystemLibrary.LineTraceSingle` :`Start` _returnvalue :`End` (+ _returnvalue (* (`SceneComponent.GetForwardVector` `Origin Component`) `Grab Length`)) :`TraceChannel` "TraceTypeQuery1" :`DrawDebugType` "ForDuration"))
  (if _returnvalue_2
    (bind (_bblockinghit _binitialoverlap _time _distance _location _impactpoint _normal _impactnormal _physmat) (`GameplayStatics.BreakHitResult` _outhit))
    (`/Engine/EditorBlueprintResources/StandardMacros.IsValid` _physmat
      (:`Is Valid`
        (`KismetSystemLibrary.PrintString` (`KismetSystemLibrary.GetDisplayName` _physmat))
        (if (== _physmat "/Game/Art/Materials/Dev/PM_Climbable.PM_Climbable")
          (return _location))))))

(fn `RightHandGrab`
  (params (`Grab Length` :type "Float (single-precision)") (`Origin Component` :type "SceneComponent Object Reference"))
  (bind _grab_point (`self.RayCast` `Origin Component` `Grab Length`))
  (`self.Set RightHand` _grab_point)
  (return))

(fn `RightHandRelease`
  (`self.Set RightHand` (0.0 0.0 0.0))
  (return))

(fn `Set LeftHand`
  (params (RightHand_Loc :type "Vector Structure"))
  (set `self.LeftHand_Loc` RightHand_Loc)
  (return))

(fn `Set RightHand`
  (params (RightHand_Loc :type "Vector Structure"))
  (set `self.RightHand_Loc` RightHand_Loc)
  (return))