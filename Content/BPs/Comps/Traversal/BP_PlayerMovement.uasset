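; BP_PlayerMovement is a player traversal component with an early climb check that only prints its result so far.
; On BeginPlay it binds to the TryToClimb dispatcher on its BP_PlayerBas owner.
; When StartClimb receives a true input, it runs a debug-drawn complex Visibility trace forward from the owner.
; A blocking hit with the PM_Climbable physical material counts as climbable.
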(event `self.ReceiveBeginPlay`
  (bind _asbp_player_bas (cast `/Game/BPs/Player/BP_PlayerBas` (`self.GetOwner`)))
  (add `/Game/BPs/Player/BP_PlayerBas.TryToClimb` _asbp_player_bas (`|CreateDelegate` :!event `StartClimb`))
  (`KismetSystemLibrary.PrintString` "Hello"))

(event `StartClimb`
  (params (ActionValue :type Boolean))
  (if ActionValue
    (bind _outhit (`self.ClimbingLineTrace`))
    (bind (_bblockinghit _binitialoverlap _time _distance _location _impactpoint _normal _impactnormal _physmat) (`GameplayStatics.BreakHitResult` _outhit))
    (if (and _bblockinghit (== _physmat "/Game/Art/Materials/Dev/PM_Climbable.PM_Climbable"))
      (`KismetSystemLibrary.PrintString` "Can Climb")
      (else
        (`KismetSystemLibrary.PrintString` "No Climb")))))

(fn `ClimbingLineTrace`
  (returns (OutHit :type "HitResult Structure"))
  (bind _returnvalue (`self.GetOwner`))
  (bind _returnvalue_2 (`Actor.K2_GetActorLocation` _returnvalue))
  (bind _outhit (`KismetSystemLibrary.LineTraceSingle` :`Start` _returnvalue_2 :`End` (+ _returnvalue_2 (* (`KismetMathLibrary.GetForwardVector` (`Actor.K2_GetActorRotation` _returnvalue)) (`self.ClimbLineTrace`))) :`TraceChannel` "TraceTypeQuery1" :`bTraceComplex` true :`DrawDebugType` "ForDuration"))
  (return _outhit))