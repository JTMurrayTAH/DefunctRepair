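; Actor component that adds a keycard requirement, checking whether a given actor holds a key of the required KeyLevel.
; CheckIfKeyMatches finds the actor's BP_AC_Keys component and looks up KeyLevel in its KeyInventory.
; A non-zero count consumes the key through RemoveKey and fires the KeySuccess dispatcher, otherwise KeyFailure fires.
; An actor without a keys component triggers neither dispatcher.
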(event `CheckIfKeyMatches`
  (params (KeyOwner :type "Actor Object Reference"))
  (bind _returnvalue (`Actor.GetComponentByClass` KeyOwner "/Game/BPs/Player/BP_AC_Keys.BP_AC_Keys_C"))
  (`/Engine/EditorBlueprintResources/StandardMacros.IsValid` _returnvalue
    (:`Is Valid`
      (if (!= (`BlueprintMapLibrary.Map_Find` (`/Game/BPs/Player/BP_AC_Keys.KeyInventory` _returnvalue) (`self.KeyLevel`)) 0)
        (`/Game/BPs/Player/BP_AC_Keys.RemoveKey` _returnvalue (`self.KeyLevel`))
        (`self.ED_KeySuccess` null)
        (else
          (`self.ED_KeyFailure` null))))))